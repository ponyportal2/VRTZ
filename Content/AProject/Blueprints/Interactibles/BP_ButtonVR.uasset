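; BP_ButtonVR is a VR push button that a motion controller presses by overlapping it.
; On overlap it tracks the controller's movement projected onto the button's up axis, using the absolute distance to sink the button up to a maximum travel.
; At full travel it calls Pressed and prints a debug string.
; A full press or the tracked controller leaving starts an interpolated return to the initial position.
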(event OnComponentBeginOverlap(VRButton)
  (params (OverlappedComponent :type Primitive%20Component%20Object%20Reference) (OtherActor :type Actor%20Object%20Reference) (OtherComp :type Primitive%20Component%20Object%20Reference) (OtherBodyIndex :type Integer) (bFromSweep :type Boolean) (SweepResult :type Hit%20Result%20Structure%20%28by%20ref%29))
  (if (and (not (Variables|Default|GetbIsTracking)) (not (Variables|Default|GetIsReturning)))
    (bind _asbp_motion_controller (Utilities|Casting|CastToBP_MotionController OtherActor))
    (Variables|Default|SetTrackingMC (Variables|/Game/VirtualRealityBP/Blueprints/BP_MotionController.BP_MotionController_C|GetMotionController _asbp_motion_controller))
    (Variables|Default|SetbIsTracking true)
    (Variables|Default|SetMCInitialLocation (Transformation|GetWorldLocation (Variables|Default|GetTrackingMC)))
    (Variables|Default|SetButtonInitialLocation (Transformation|GetWorldLocation (Variables|Default|GetVRButton)))))

(event OnComponentEndOverlap(VRButton)
  (params (OverlappedComponent :type Primitive%20Component%20Object%20Reference) (OtherActor :type Actor%20Object%20Reference) (OtherComp :type Primitive%20Component%20Object%20Reference) (OtherBodyIndex :type Integer))
  (bind _asbp_motion_controller (Utilities|Casting|CastToBP_MotionController OtherActor))
  (if (== (Variables|/Game/VirtualRealityBP/Blueprints/BP_MotionController.BP_MotionController_C|GetMotionController _asbp_motion_controller) (Variables|Default|GetTrackingMC))
    (Variables|Default|SetbIsTracking false)
    (Variables|Default|SetIsReturning true)))

(event Custom|FullyPressed
  (Variables|Default|SetbIsTracking false)
  (Variables|Default|SetIsReturning true)
  (Default|CallPressed)
  (Development|PrintString "Hello"))

(event EventBeginPlay)

(event Collision|EventActorBeginOverlap
  (params (OtherActor :type Actor%20Object%20Reference)))

(event EventTick
  (params (DeltaSeconds :type Float%20%28single-precision%29))
  (if (Variables|Default|GetbIsTracking)
    (Variables|Default|SetCurrentTravel (Math|Float|Clamp(Float) (Math|Float|Absolute(Float) (Math|Vector|VectorLength (Math|Vector|ProjectVectorontoVector (- (Transformation|GetWorldLocation (Variables|Default|GetTrackingMC)) (Variables|Default|GetMCInitialLocation)) (Math|Vector|GetUpVector (Variables|Default|GetVRButton))))) 0.0 (Variables|Default|GetMax%20Travel)))
    (bind _output_get (Variables|Default|SetButtonCurrentLocation (- (Variables|Default|GetButtonInitialLocation) (* (Math|Vector|GetUpVector (Variables|Default|GetVRButton)) (Variables|Default|GetCurrentTravel)))))
    (Transformation|SetWorldLocation (Variables|Default|GetVRButton) _output_get false false)
    (if (>= (Variables|Default|GetCurrentTravel) (Variables|Default|GetMax%20Travel))
      (CallFunction|FullyPressed))
    (elif (Variables|Default|GetIsReturning)
      (bind _output_get_2 (Variables|Default|SetButtonCurrentLocation (Math|Interpolation|VInterpTo (Variables|Default|GetButtonCurrentLocation) (Variables|Default|GetButtonInitialLocation) (Utilities|Time|GetWorldDeltaSeconds) (Variables|Default|GetButtonReturnSpeed))))
      (Transformation|SetWorldLocation (Variables|Default|GetVRButton) _output_get_2 false false)
      (if (Class|KismetMathLibrary|EqualExactlyVectorVector (Variables|Default|GetButtonCurrentLocation) (Variables|Default|GetButtonInitialLocation))
        (Variables|Default|SetIsReturning false)))))

(fn ConstructionScript)