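; Physical push button interactible whose cap is pushed down by whatever component overlaps it.
; On begin overlap it stores the component and its starting location, clearing the component when that same one leaves.
; Each tick, the component's downward travel in the base's local space, clamped to a maximum, offsets the cap.
; Without an overlap, the cap interpolates back to rest; no press event is fired.
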(event OnComponentBeginOverlap(ButtonComponent)
  (params (OverlappedComponent :type Primitive%20Component%20Object%20Reference) (OtherActor :type Actor%20Object%20Reference) (OtherComp :type Primitive%20Component%20Object%20Reference) (OtherBodyIndex :type Integer) (bFromSweep :type Boolean) (SweepResult :type Hit%20Result%20Structure%20%28by%20ref%29))
  (bind _output_get (Variables|Default|SetOverlappedComponent OtherComp))
  (Variables|Default|SetInitialOverlapLocation (Transformation|GetWorldLocation _output_get)))

(event OnComponentEndOverlap(ButtonComponent)
  (params (OverlappedComponent :type Primitive%20Component%20Object%20Reference) (OtherActor :type Actor%20Object%20Reference) (OtherComp :type Primitive%20Component%20Object%20Reference) (OtherBodyIndex :type Integer))
  (if (== OtherComp (Variables|Default|GetOverlappedComponent))
    (Variables|Default|SetOverlappedComponent 0)))

(event EventBeginPlay)

(event Collision|EventActorBeginOverlap
  (params (OtherActor :type Actor%20Object%20Reference)))

(event EventTick
  (params (DeltaSeconds :type Float%20%28single-precision%29))
  (Variables|Default|GetOverlappedComponent
    (:then
      (bind _output_get (Variables|Default|SetButtonPressedAmount (Math|Float|Clamp(Float) (.z (- (Math|Transform|InverseTransformLocation (Transformation|GetWorldTransform (Variables|Default|GetButtonBase)) (Variables|Default|GetInitialOverlapLocation)) (Math|Transform|InverseTransformLocation (Transformation|GetWorldTransform (Variables|Default|GetButtonBase)) (Transformation|GetWorldLocation (Variables|Default|GetOverlappedComponent))))) 0.0 (Variables|Default|GetMaxButtonPressedAmount))))
      (Transformation|SetRelativeLocation (Variables|Default|GetButtonComponent) (Math|Vector|MakeVector 0.0 0.0 (* _output_get -1.0)) false false))
    (:else
      (Transformation|SetRelativeLocation (Variables|Default|GetButtonComponent) (Math|Interpolation|VInterpTo (Variables|/Script/Engine.SceneComponent|GetRelativeLocation (Variables|Default|GetButtonComponent)) "0, 0, 0" (Utilities|Time|GetWorldDeltaSeconds) (Variables|Default|GetBounce)) false false))))

(fn ConstructionScript)